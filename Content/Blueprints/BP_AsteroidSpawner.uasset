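; BP_AsteroidSpawner is an actor that spawns moving BP_Asteroid actors around the player pawn.
; BeginPlay starts a looping timer on the function named in SpawnFuncionName and stores its handle.
; SpawnAsteroid places each asteroid at a random direction and bounded distance from the player, then sets a random-speed velocity.
; That velocity re-rolls the random offset, so its direction is random rather than aimed from the spawn point at the player.
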(event EventBeginPlay
  (bind _returnvalue (Utilities|Time|SetTimerbyFunctionName 0 (Variables|Default|GetSpawnFuncionName) 2.0 true))
  (Variables|Default|SetTimerHandle_Spawner _returnvalue))

(event Collision|EventActorBeginOverlap
  (params (OtherActor :type Actor%20Object%20Reference)))

(event EventTick
  (params (DeltaSeconds :type Float%20%28single-precision%29)))

(fn ConstructionScript)

(fn SpawnAsteroid
  (bind _returnvalue (Game|Player|GetPlayerPawn 0))
  (bind _returnvalue_2 (Math|Random|RandomUnitVector))
  (bind _minspawnrange (Variables|Default|GetMinSpawnRange))
  (bind _maxspawnrange (Variables|Default|GetMaxSpawnRange))
  (bind _returnvalue_3 (Transformation|GetActorLocation _returnvalue))
  (bind _returnvalue_4 (Math|Random|RandomFloatinRange _minspawnrange _maxspawnrange))
  (bind _returnvalue_5 (* _returnvalue_2 _returnvalue_4))
  (bind _returnvalue_6 (+ _returnvalue_3 _returnvalue_5))
  (bind _returnvalue_7 (Game|SpawnActorfromClass "/Game/Blueprints/Asteroids/BP_Asteroid.BP_Asteroid_C" (Math|Transform|MakeTransform _returnvalue_6 "0, 0, 0" "1,1,1") "AdjustIfPossibleButAlwaysSpawn" 0 0))
  (Class|A3DAsteroid|SetVelocityVector _returnvalue_7 (* (Math|Vector|Normalize (- _returnvalue_3 _returnvalue_6)) (Math|Random|RandomFloatinRange (Variables|Default|GetMinAsteroidSpeed) (Variables|Default|GetMaxAsteroidSpeed)))))