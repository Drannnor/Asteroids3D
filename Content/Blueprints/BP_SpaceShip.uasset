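; BP_SpaceShip is a spaceship Blueprint that displays its health on a WBP_HealthBar widget.
; On BeginPlay it caches the widget from its HealthBar component and seeds it with the HealthComponent's current and maximum health, plus the ship's bar color.
; The HealthComponent's OnHealthChanged event then pushes new values to the widget, so the bar updates by event without using Tick.
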(event OnHealthChanged(HealthComponent)
  (params (HealthComp :type A3D%20Health%20Component%20Object%20Reference) (Health :type Float%20%28single-precision%29) (HealthDelta :type Float%20%28single-precision%29) (DamageType :type Damage%20Type%20Object%20Reference) (InstigatedBy :type Controller%20Object%20Reference) (DamageCauser :type Actor%20Object%20Reference))
  (bind _as_wbp_health_bar (Variables|Default|GetAs%20WBP%20Health%20Bar))
  (Variables|/Game/UI/WBP_HealthBar.WBP_HealthBar_C|SetHealth _as_wbp_health_bar Health)
  (Variables|/Game/UI/WBP_HealthBar.WBP_HealthBar_C|SetMaxHealth _as_wbp_health_bar (Variables|/Script/Asteroid3D_VVRTest.A3D_HealthComponent|GetMaxHealth HealthComp)))

(event EventBeginPlay
  (bind _healthcomponent (Variables|Default|GetHealthComponent))
  (bind _aswbp_health_bar (Utilities|Casting|CastToWBP_HealthBar (UserInterface|GetUserWidgetObject (Variables|Default|GetHealthBar))))
  (bind _output_get (Variables|Default|SetAs%20WBP%20Health%20Bar _aswbp_health_bar))
  (Variables|/Game/UI/WBP_HealthBar.WBP_HealthBar_C|SetMaxHealth _output_get (Variables|/Script/Asteroid3D_VVRTest.A3D_HealthComponent|GetMaxHealth _healthcomponent))
  (Variables|/Game/UI/WBP_HealthBar.WBP_HealthBar_C|SetHealth _output_get (Variables|/Script/Asteroid3D_VVRTest.A3D_HealthComponent|GetHealth _healthcomponent))
  (Variables|/Game/UI/WBP_HealthBar.WBP_HealthBar_C|SetBarColor _output_get (Variables|Default|GetBar%20Color)))

(event Collision|EventActorBeginOverlap
  (params (OtherActor :type Actor%20Object%20Reference)))

(event EventTick
  (params (DeltaSeconds :type Float%20%28single-precision%29)))

(fn ConstructionScript)